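; AI controller for the Alien1 NPC that runs its behavior tree and records the pawn's spawn location in the blackboard on BeginPlay.
; State setters for passive, investigating, seeking, attacking and dead write the state enum plus any move-to, point-of-interest or target data to the blackboard, then notify the pawn of the change.
; GetNPCState reads the blackboard state, while GetIsDead and GetTeamID are stubs returning false.
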(event EventTick
  (params (DeltaSeconds :type Float%20%28single-precision%29)))

(event EventBeginPlay
  (Class|AIController|UseBlackboard "/Game/FPSGame/NPC/Alien1/AI/Alien1_BB.Alien1_BB")
  (AI|RunBehaviorTree "/Game/FPSGame/NPC/Alien1/AI/Alien1_BT.Alien1_BT")
  (AI|Components|Blackboard|SetValueasVector (Variables|Default|GetBlackboard) (Utilities|Name|MakeLiteralName "SpawnLocation") (Transformation|GetActorLocation (Pawn|GetControlledPawn))))

(fn ConstructionScript)

(fn GetNPCState
  (return (Utilities|Enum|ByteToEnumNPC_State (Class|BlackboardComponent|GetValueasEnum (Variables|Default|GetBlackboard) (Variables|Keys|GetStateKey)))))

(fn SetStateasPassive
  (bind _returnvalue (Utilities|Enum|LiteralenumNPC_State "NewEnumerator0"))
  (AI|Components|Blackboard|SetValueasEnum (Variables|Default|GetBlackboard) (Variables|Keys|GetStateKey) _returnvalue)
  (Class|BPIAIHelper|NotifyStateChanged(Message) (Pawn|GetControlledPawn) _returnvalue))

(fn SetStateasInvestigating
  (params (MoveToLocation :type Vector) (PointOfInterest :type Vector))
  (bind _returnvalue (Utilities|Enum|LiteralenumNPC_State "NewEnumerator1"))
  (AI|Components|Blackboard|SetValueasEnum (Variables|Default|GetBlackboard) (Variables|Keys|GetStateKey) _returnvalue)
  (AI|Components|Blackboard|SetValueasVector (Variables|Default|GetBlackboard) (Variables|Default|GetMoveToKey) MoveToLocation)
  (AI|Components|Blackboard|SetValueasVector (Variables|Default|GetBlackboard) (Variables|Default|GetPOIKey) PointOfInterest)
  (Class|BPIAIHelper|NotifyStateChanged(Message) (Pawn|GetControlledPawn) _returnvalue))

(fn SetStateasSeeking
  (params (Search :type Vector))
  (bind _returnvalue (Utilities|Enum|LiteralenumNPC_State "NewEnumerator2"))
  (AI|Components|Blackboard|SetValueasEnum (Variables|Default|GetBlackboard) (Variables|Keys|GetStateKey) _returnvalue)
  (AI|Components|Blackboard|SetValueasVector (Variables|Default|GetBlackboard) (Variables|Default|GetMoveToKey) Search)
  (Class|BPIAIHelper|NotifyStateChanged(Message) (Pawn|GetControlledPawn) _returnvalue))

(fn SetStateasAttacking
  (params (TargetIn :type Actor%20Object%20Reference))
  (bind _returnvalue (Utilities|Enum|LiteralenumNPC_State "NewEnumerator3"))
  (AI|Components|Blackboard|SetValueasEnum (Variables|Default|GetBlackboard) (Variables|Keys|GetStateKey) _returnvalue)
  (AI|Components|Blackboard|SetValueasObject (Variables|Default|GetBlackboard) (Variables|Default|GetEnemyTargetKey) TargetIn)
  (Class|BPIAIHelper|NotifyStateChanged(Message) (Pawn|GetControlledPawn) _returnvalue))

(fn SetStateasDead
  (bind _returnvalue (Utilities|Enum|LiteralenumNPC_State "NewEnumerator4"))
  (AI|Components|Blackboard|SetValueasEnum (Variables|Default|GetBlackboard) (Variables|Keys|GetStateKey) _returnvalue)
  (Class|BPIAIHelper|NotifyStateChanged(Message) (Pawn|GetControlledPawn) _returnvalue))

(fn GetIsDead
  (return false))

(fn GetTeamID
  (return false))
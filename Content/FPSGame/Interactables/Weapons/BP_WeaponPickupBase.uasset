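; Base Blueprint for a weapon pickup that bobs in the world and hands its weapon to the player on interaction.
; BeginPlay caches the BP_Player reference, and InteractWithWeapon passes WeaponToSpawn to that player's WeaponPickup.
; A DoOnce then limits the pickup sound and self-destruction to a single run.
; Tick plays the Oscillate timeline, whose output is added as a local offset on each update.
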(event Custom|InteractWithWeapon
  ;[0 0.5 0.06307] Runs event in BP_Player
  (Default|WeaponPickup (Variables|Default|GetPlayer) (Variables|Default|GetWeaponToSpawn))
  (Utilities|FlowControl|DoOnce false
    (:Completed
      (Audio|PlaySound2D (Variables|Default|GetPickupSound) 1.0 1.0 0.0 0 0)
      (Actor|DestroyActor))))

(event EventBeginPlay
  ;[0.1336 1 0.1188] Reference to player
  (bind _asbp_player (Utilities|Casting|CastToBP_Player (Game|GetPlayerCharacter 0)))
  (Variables|Default|SetPlayer _asbp_player))

(event EventTick
  (params (DeltaSeconds :type Float%20%28single-precision%29))
  ;[0 0.5 0.06307] Weapon oscillate in world
  (bind _oscilate_anim (Timeline|Oscillate Play)
    (:Update
      (Transformation|AddActorLocalOffset _oscilate_anim false false))))

(fn ConstructionScript)
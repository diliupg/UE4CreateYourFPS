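; Alien2 enemy character that chases the player on sight via AIMoveTo and plays a throw-attack montage on reaching them.
; Bullet damage scales by the hit physical material, explosive damage by distance; both feed a shared health update.
; Hits spawn screen-projected damage numbers, plus hit markers for direct shots.
; Death triggers ragdoll, kill sound and a weapon-based impulse, then removes the capsule and destroys the actor after a delay.
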(event OnSeePawn(PawnSensing)
  (params (Pawn :type Pawn%20Object%20Reference))
  (Variables|Default|SetIsSeeingPlayer? true)
  (CallFunction|FollowPlayer))

(event Custom|FollowPlayer
  (Variables|Default|SetCanAttack? true)
  (if (Variables|Default|GetIsSeeingPlayer?)
    (AI|AIMoveTo self "0, 0, 0" (Variables|Default|GetPlayer) 2e+02 false
      (:OnSuccess
        (if (Variables|Default|GetCanAttack?)
          (Variables|Default|SetCanAttack? false)
          (bind _returnvalue (Animation|PlayAnimMontage "/Game/FPSGame/NPC/Alien2/Animations/AM_Alien2ThrowAttack.AM_Alien2ThrowAttack" 1.0 "None"))
          (Utilities|FlowControl|Delay _returnvalue)
          (Variables|Default|SetCanAttack? true))))
    (else
      (Variables|Default|SetIsSeeingPlayer? false))))

(event EventBeginPlay
  ;[0.05084 0.01528 0.0625] Get reference to player
  (bind _asbp_player (Utilities|Casting|CastToBP_Player (Game|GetPlayerCharacter 0)))
  (Variables|Default|SetPlayer _asbp_player))

(event EventEnemyTakeDamage
  (params (WeaponStats :type S%20Weapon%20Stats%20Structure) (HitResult :type Hit%20Result%20Structure))
  (bind (_bblockinghit _binitialoverlap _time _distance _location _impactpoint _normal _impactnormal _physmat _hitactor _hitcomponent _hitbonename) (Collision|BreakHitResult HitResult))
  ;[0.007035 0.003031 0.01042] Enemy takes damage
  (if (not (Variables|Default|GetIsDead?))
    (bind _calculateddamage (CallFunction|CalculateDamage (.Damage (Utilities|Struct|BreakS_WeaponStats WeaponStats)) HitResult self))
    (bind (_isdead _newcurrenthealth) (CallFunction|HealthUpdate _calculateddamage (Variables|Default|GetCurrentHealth)))
    (Variables|Default|SetCurrentHealth _newcurrenthealth)
    (bind _output_get (Variables|Default|SetIsDead? _isdead))
    (if _output_get
      (CallFunction|EnemyDeath _impactpoint _hitbonename))
    (CallFunction|DamageNumbers _calculateddamage _impactpoint (Utilities|Enum|Equal(Enum) (Variables|/Script/PhysicsCore.PhysicalMaterial|GetSurfaceType _physmat) "SurfaceType1"))
    (Utilities|IsValid (Variables|Default|GetHitMarkerRef)
      (:Is%20Valid
        (Widget|RemovefromParent (Variables|Default|GetHitMarkerRef)) ; Removes previous HitMarker if another hit occurs beore the first disappears
      )
      (:Is%20Not%20Valid
        _))
    ;[0.3177 0.1485 0] Add hit markers if enemy still alive
    (bind _returnvalue (UserInterface|CreateWidget "/Game/FPSGame/UI/HitMarkers.HitMarkers_C" 0 (Variables|Default|GetIsDead?)))
    (bind _output_get_2 (Variables|Default|SetHitMarkerRef _returnvalue))
    (UserInterface|Viewport|AddtoViewport _output_get_2 0)))

(event EventDamageNumbers
  (params (Damage :type Float%20%28single-precision%29) (ImpactLocation :type Vector :default "0, 0, 0") (HeadShot :type Boolean))
  (bind _returnvalue (Game|GetPlayerController 0))
  (bind _screenposition (Class|WidgetLayoutLibrary|ProjectWorldLocationtoWidgetPosition _returnvalue ImpactLocation false))
  (bind (_x _y) (Math|Vector2D|BreakVector2D _screenposition))
  (bind _returnvalue_2 (UserInterface|CreateWidget "/Game/FPSGame/UI/DamageNumbers.DamageNumbers_C" 0 Damage HeadShot))
  (Class|Widget|SetRenderTranslation (Variables|/Game/FPSGame/UI/DamageNumbers.DamageNumbers_C|GetSizeBox_114 _returnvalue_2) (Math|Vector2D|MakeVector2D (+ (+ _x -1e+02) (Math|Random|RandomFloatinRange -25.0 1.5e+02)) (+ (+ _y -1e+02) (Math|Random|RandomFloatinRange 0.0 5e+01))))
  (UserInterface|Viewport|AddtoViewport _returnvalue_2 0))

(event EventTakeRadialDamage
  (params (HitResult :type Hit%20Result%20Structure) (WeaponStats :type S%20Weapon%20Stats%20Structure))
  (bind (_damage _imapctradius) (Utilities|Struct|BreakS_WeaponStats WeaponStats))
  (bind (_bblockinghit _binitialoverlap _time _distance _location _impactpoint _normal _impactnormal _physmat _hitactor _hitcomponent _hitbonename) (Collision|BreakHitResult HitResult))
  ;[0.07035 0.03031 0.1042] Enemy takes radial (explosive) damage
  (if (not (Variables|Default|GetIsDead?))
    (bind _appliedradialdamage (CallFunction|CalculateRadialDamage _damage _imapctradius _impactpoint))
    (bind _isdead (CallFunction|HealthUpdate _appliedradialdamage))
    (if _isdead
      (CallFunction|EnemyDeath _impactpoint _hitbonename)
      (else
        (CallFunction|DamageNumbers _appliedradialdamage _impactpoint false)))))

(event EventTick
  (params (DeltaSeconds :type Float%20%28single-precision%29))
  (if (Variables|Default|GetIsSeeingPlayer?)
    _
    (else
      (Components|Movement|StopMovementImmediately (Variables|Character|GetCharacterMovement))))
  (if (Variables|Default|GetIsDead?)
    (Utilities|FlowControl|Delay 15.0)
    (Actor|DestroyActor)))

(fn ConstructionScript)

(fn CalculateDamage
  (params (Damage :type Float%20%28single-precision%29) (HitResult :type Hit%20Result%20Structure))
  ;[0.006247 0.04143 0.07812] Decide which part of the body was hit by checking the physics material
  (LocalVariables|SetLocalDamage Damage)
  (return (* (LocalVariables|GetLocalDamage) (Variables|/Script/PhysicsCore.PhysicalMaterial|GetDestructibleDamageThresholdScale (.PhysMat (Collision|BreakHitResult HitResult))))))

(fn HealthUpdate
  (params (DamageApplied :type Float%20%28single-precision%29))
  (Utilities|FlowControl|Sequence
    (:then_0
      (if (>= DamageApplied (Variables|Default|GetCurrentHealth))
        (LocalVariables|SetLocalIsDead? true)
        (Variables|Default|SetCurrentHealth 0.0)
        (else
          (Variables|Default|SetCurrentHealth (- (Variables|Default|GetCurrentHealth) DamageApplied)))))
    (:then_1
      (return (LocalVariables|GetLocalIsDead?)))))

(fn EnemyDeath
  (params (HitLocation :type Vector) (BoneName :type Name))
  (bind _capsulecomponent (Variables|Collision|GetCapsuleComponent))
  (bind _player (Variables|Default|GetPlayer))
  (Utilities|FlowControl|Sequence
    (:then_0
      ;[0 0.02795 0.2656] Enabling Ragdoll physics
      (Physics|SetSimulatePhysics (Variables|Character|GetMesh) true)
      (Pawn|Components|CharacterMovement|DisableMovement (Variables|Character|GetCharacterMovement)))
    (:then_1
      (Audio|PlaySound2D "/Game/FPSGame/Audio/kill-sound.kill-sound" 1.0 1.0 0.0 0 0))
    (:then_2
      (Physics|AddImpulseatLocation (Variables|Character|GetMesh) (* (Math|Vector|GetUnitDirection(Vector) (Transformation|GetActorLocation _player) (Transformation|GetActorLocation)) (Variables|/Game/FPSGame/Weapons/BP_WeaponBase.BP_WeaponBase_C|GetKillImpulse (Variables|/Game/FPSGame/_PlayerCharacter/BP_Player.BP_Player_C|GetCurrentWeapon _player))) HitLocation BoneName)
      (if (Utilities|IsValid _capsulecomponent)
        (Components|DestroyComponent _capsulecomponent)
        (Variables|Default|SetIsDead? true)
        (Variables|Default|SetTags self (Variables|Default|GetTag_Dead))))))

(fn CalculateRadialDamage
  (params (Damage :type Float%20%28single-precision%29) (ImpaceRadius :type Float%20%28single-precision%29) (ImpactPoint :type Vector))
  (LocalVariables|SetLocalDamage Damage)
  (return (Math|Float|Clamp(Float) (* (- 1.0 (/ (Math|Vector|VectorLength (- ImpactPoint (Transformation|GetActorLocation))) ImpaceRadius)) (LocalVariables|GetLocalDamage)) 0.0 (LocalVariables|GetLocalDamage))))
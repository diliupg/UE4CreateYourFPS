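; BP_Alien1 is an alien enemy NPC for an FPS, currently a skeleton with most behavior unimplemented.
; On BeginPlay it caches the BP_Player reference, then spawns its weapon class and snaps it to the mesh's WeaponSocket.
; Shooting and damage events are empty stubs.
; Death state is read from HealthComponent, and the team ID getter returns a constant false.
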(event OnDamageTaken(HealthComponent))

(event Custom|StartShooting)

(event EventBeginPlay
  (bind _self self)
  ;[0.01054 0.09375 0.01876] Reference to player
  (bind _asbp_player (Utilities|Casting|CastToBP_Player (Game|GetPlayerCharacter 0)))
  (Variables|Default|SetPlayer _asbp_player)
  (bind _returnvalue (Game|SpawnActorfromClass (Variables|Default|GetWeaponClass) (CallFunction|IdentityTransform) "AlwaysSpawn" _self _self))
  (bind _output_get (Variables|Default|SetWeapon _returnvalue))
  (Transformation|AttachComponentToComponent _output_get (Variables|Character|GetMesh) "WeaponSocket" "SnapToTarget" "SnapToTarget" "SnapToTarget" true))

(event EventEnemyTakeDamage
  (params (WeaponStats :type S%20Weapon%20Stats%20Structure) (HitResult :type Hit%20Result%20Structure))
  (if (not (Variables|Default|GetIsDead?))
    _))

(fn ConstructionScript)

(fn GetIsDead
  (return (Default|IsDead (Variables|Default|GetHealthComponent))))

(fn GetTeamID
  (return false))